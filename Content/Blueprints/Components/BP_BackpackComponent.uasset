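; Backpack component for characters that stores quest items, consumable items and available weapons with their reserve ammo.
; On BeginPlay it restores all three collections from the game instance's save object, only for a player character outside a new game.
; Ammo updates clamp the reserve, return rounds to load when decreasing, and notify the current weapon.
; Adding a weapon registers zero ammo and updates the owner's current weapon; consumable add/remove are empty stubs.
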(event EventBeginPlay
  (CallFunction|ConfigureBackpack))

(fn AddQuestItem
  (params (InItemName :type Name))
  (Utilities|Set|Add (Variables|Default|GetQuestItems) InItemName))

(fn RemoveQuestItem
  (params (InItemName :type Name))
  (bind _returnvalue (Utilities|Set|Remove (Variables|Default|GetQuestItems) InItemName))
  (return _returnvalue))

(fn AddConsunableItem)

(fn RemoveConsunableItem)

(fn UpdateAmmobyName
  (params (InWeaponName :type Name) (InAmmo :type Integer) (InIncreased :type Boolean))
  (bind _avalableweapon (Variables|Default|GetAvalableWeapon))
  (bind (_value _returnvalue) (Utilities|Map|Find _avalableweapon InWeaponName))
  (bind _asbp_character_base (Utilities|Casting|CastToBP_CharacterBase (Components|GetOwner)))
  (bind _currentweapon (Variables|/Game/Blueprints/Characters/BP_CharacterBase.BP_CharacterBase_C|GetCurrentWeapon _asbp_character_base)
    (:then
      (LocalVariables|SetL_CurrentWeapon _currentweapon)
      (if _returnvalue
        (LocalVariables|SetL_AmmoInBackpackCurrent _value)
        (Utilities|FlowControl|Sequence
          (:then_0
            (if InIncreased
              (Utilities|FlowControl|Sequence
                (:then_0
                  (if (<= (LocalVariables|GetL_AmmoInBackpackCurrent) 0)
                    (if (<= (Variables|/Game/Blueprints/Weapons/BP_WeaponBase.BP_WeaponBase_C|GetRoundsCurrent (LocalVariables|GetL_CurrentWeapon)) 0)
                      (Variables|/Game/Blueprints/Weapons/BP_WeaponBase.BP_WeaponBase_C|SetWeaponState (LocalVariables|GetL_CurrentWeapon) "NewEnumerator2"))))
                (:then_1
                  (LocalVariables|SetL_Current (+ (LocalVariables|GetL_AmmoInBackpackCurrent) InAmmo))
                  (if (< (LocalVariables|GetL_Current) (Utilities|Struct|BreakSTRUCT_WeaponStats (Variables|/Game/Blueprints/Weapons/BP_WeaponBase.BP_WeaponBase_C|GetWeaponStats (LocalVariables|GetL_CurrentWeapon))))
                    (LocalVariables|SetL_AmmoInBackpackCurrent (LocalVariables|GetL_Current))
                    (else
                      (LocalVariables|SetL_AmmoInBackpackCurrent (Utilities|Struct|BreakSTRUCT_WeaponStats (Variables|/Game/Blueprints/Weapons/BP_WeaponBase.BP_WeaponBase_C|GetWeaponStats (LocalVariables|GetL_CurrentWeapon))))))))
              (else
                (LocalVariables|SetL_Current (- (LocalVariables|GetL_AmmoInBackpackCurrent) InAmmo))
                (if (> (LocalVariables|GetL_Current) 0)
                  (LocalVariables|SetL_AmmoInBackpackCurrent (LocalVariables|GetL_Current))
                  (LocalVariables|SetL_Current (Utilities|Struct|BreakSTRUCT_WeaponStats (Variables|/Game/Blueprints/Weapons/BP_WeaponBase.BP_WeaponBase_C|GetWeaponStats (LocalVariables|GetL_CurrentWeapon))))
                  (else
                    (LocalVariables|SetL_AmmoInBackpackCurrent 0)
                    (LocalVariables|SetL_Current (+ (Utilities|Struct|BreakSTRUCT_WeaponStats (Variables|/Game/Blueprints/Weapons/BP_WeaponBase.BP_WeaponBase_C|GetWeaponStats (LocalVariables|GetL_CurrentWeapon))) (LocalVariables|GetL_Current))))))))
          (:then_1
            (Utilities|Map|Add (Variables|Default|GetAvalableWeapon) InWeaponName (LocalVariables|GetL_AmmoInBackpackCurrent)))
          (:then_2
            (Default|CallOnWeaponStatusChanged (LocalVariables|GetL_CurrentWeapon))
            (return (LocalVariables|GetL_Current))))
        (else
          (Default|CallOnWeaponStatusChanged (LocalVariables|GetL_CurrentWeapon))
          (return 0))))
    (:else)))

(fn GetAmmoforWeapon
  (params (InWeaponName :type Name%20%28by%20ref%29))
  (bind _avalableweapon (Variables|Default|GetAvalableWeapon))
  (bind (_value _returnvalue) (Utilities|Map|Find _avalableweapon InWeaponName))
  (if _returnvalue
    (return true _value)
    (else
      (return false 0))))

(fn GetMaxRoundsforWeapon
  (params (InWeaponName :type Name))
  (bind _returnvalue (Utilities|GetDataTableRow "/Game/Data/DT_WeaponStats.DT_WeaponStats" InWeaponName)
    (:then
      (return true (Utilities|Struct|BreakSTRUCT_WeaponStats _returnvalue)))
    (:RowNotFound
      (return false 0))))

(fn AddWeaponItem
  (params (InWeaponName :type Name))
  (Utilities|Map|Add (Variables|Default|GetAvalableWeapon) InWeaponName 0)
  (bind _asbp_character_base (Utilities|Casting|CastToBP_CharacterBase (Components|GetOwner)))
  (Default|UpdateCurrentWeapon _asbp_character_base InWeaponName))

(fn ConfigureBackpack
  (bind _savegameobject (Utilities|CheckSaveGame)
    (:Is%20Valid
      (LocalVariables|SetL_Save _savegameobject)
      (Utilities|FlowControl|Sequence
        (:then_0
          (Variables|Default|SetQuestItems (Variables|/Game/Blueprints/Objects/BP_SaveGame.BP_SaveGame_C|GetSavedQuestItems (LocalVariables|GetL_Save))))
        (:then_1
          (Variables|Default|SetConsunableItems (Variables|/Game/Blueprints/Objects/BP_SaveGame.BP_SaveGame_C|GetSavedConsumableItems (LocalVariables|GetL_Save))))
        (:then_2
          (Variables|Default|SetAvalableWeapon (Variables|/Game/Blueprints/Objects/BP_SaveGame.BP_SaveGame_C|GetSavedAvalableWeapon (LocalVariables|GetL_Save))))
        (:then_3
          (bind _asbp_player_character (Utilities|Casting|CastToBP_PlayerCharacter (Components|GetOwner)))
          (bind _currentweapon (Variables|/Game/Blueprints/Characters/BP_CharacterBase.BP_CharacterBase_C|GetCurrentWeapon _asbp_player_character)
            (:then
              (Default|CallOnWeaponStatusChanged _currentweapon))
            (:else)))))))