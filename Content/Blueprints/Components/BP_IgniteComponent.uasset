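; Actor component that sets its owner on fire, dealing damage over time.
; StartIgniteDamage stores damage, duration, period and causer, then runs a looping timer for periodic ApplyDamage with BP_DamageObject, plus a one-shot timer to end it.
; Re-igniting while active restarts the duration and updates damage and causer instead of stacking, but the running tick keeps its original period.
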(event Custom|StartIgniteDamage
  (params (InDamage :type Float%20%28double-precision%29) (InTime :type Float%20%28double-precision%29) (InPeriod :type Float%20%28double-precision%29) (DamageCauser :type Actor%20Object%20Reference))
  (Variables|Default|SetIgniteDamage InDamage)
  (Variables|Default|SetDamageTime InTime)
  (Variables|Default|SetDamagePeriod InPeriod)
  (Variables|Default|SetDamageCauser DamageCauser)
  (if (not (Utilities|Time|IsValidTimerHandle (Variables|Default|GetDamageTimer)))
    (bind _returnvalue (Utilities|Time|SetTimerbyEvent (EventDispatchers|CreateEvent :!event Custom|DamageCharacter) (Variables|Default|GetDamagePeriod) true))
    (Variables|Default|SetDamageTimer _returnvalue)
    (else
      (Utilities|Time|ClearandInvalidateTimerbyHandle (Variables|Default|GetDamageTimerStopper))))
  (bind _returnvalue_2 (Utilities|Time|SetTimerbyEvent (EventDispatchers|CreateEvent :!event Custom|StopDamageTimers) (Variables|Default|GetDamageTime)))
  (Variables|Default|SetDamageTimerStopper _returnvalue_2))

(event Custom|DamageCharacter
  (Game|Damage|ApplyDamage (Components|GetOwner) (Variables|Default|GetIgniteDamage) 0 (Variables|Default|GetDamageCauser) "/Game/Blueprints/Objects/BP_DamageObject.BP_DamageObject_C"))

(event Custom|StopDamageTimers
  (Utilities|Time|ClearandInvalidateTimerbyHandle (Variables|Default|GetDamageTimer))
  (Utilities|Time|ClearandInvalidateTimerbyHandle (Variables|Default|GetDamageTimerStopper)))