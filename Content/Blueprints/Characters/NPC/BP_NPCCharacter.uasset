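; NPC character Blueprint that pairs with BP_AIController and binds an overhead health bar widget to itself.
; A debug-toggled tooltip shows the controller's AI state and turns toward the player camera each tick when the player is nearby.
; Assigning a positive patrolling group switches the controller to Patrolling.
; While shooting during a chase, the weapon muzzle smoothly aims pitch and yaw at the target, resetting in other weapon states.
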(event EventBeginPlay
  (|CallParentFunction)
  (Utilities|FlowControl|Sequence
    (:then_0
      (bind _asw_health_bar (Utilities|Casting|CastToW_HealthBar (UserInterface|GetUserWidgetObject (Variables|Default|GetWidgetHP))))
      (Default|UpdateCurrentCharacterforHP _asw_health_bar self))
    (:then_1
      (Rendering|SetVisibility (Variables|Default|GetTooltipText) (Variables|Default|GetDebug) true))))

(event Collision|EventActorBeginOverlap
  (params (OtherActor :type Actor%20Object%20Reference))
  (|CallParentFunction OtherActor) ; This node is disabled and will not be called.\nDrag off pins to build functionality.
)

(event EventTick
  (params (DeltaSeconds :type Float%20%28single-precision%29))
  (|CallParentFunction DeltaSeconds)
  (Variables|Default|SetIsLookAtPlayerCamera (<= (Math|Vector|VectorLength (- (Transformation|GetWorldLocation (Variables|Default|GetCapsuleComponent)) (Transformation|GetActorLocation (Game|Player|GetPlayerPawn 0)))) 1.5e+03))
  (CallFunction|LookingatPlayerCaamera))

(fn ConstructionScript
  (|CallParentFunction))

(fn ActionMain
  (params (IsPressed :type Boolean))
  (|CallParentFunction IsPressed))

(fn LookingatPlayerCaamera
  (if (Variables|Default|GetIsLookAtPlayerCamera)
    (bind _asbp_aicontroller (Utilities|Casting|CastToBP_AIController (Pawn|GetController)))
    (bind _asbp_player_character (Utilities|Casting|CastToBP_PlayerCharacter (Game|Player|GetPlayerPawn 0)))
    (LocalVariables|SetL_CameraLocation (Transformation|GetWorldLocation (Variables|/Game/Blueprints/Characters/Player/BP_PlayerCharacter.BP_PlayerCharacter_C|GetCamera _asbp_player_character)))
    (Rendering|Components|TextRender|SetText (Variables|Default|GetTooltipText) (Utilities|Text|FormatText "{AIState}" (Utilities|String|EnumtoString (Variables|/Game/Blueprints/Controllers/BP_AIController.BP_AIController_C|GetAIState _asbp_aicontroller))))
    (Transformation|SetWorldRotation (Variables|Default|GetTooltipText) (Math|Rotator|FindLookatRotation (Transformation|GetWorldLocation (Variables|Default|GetTooltipText)) (LocalVariables|GetL_CameraLocation)) false false)))

(fn UpdatePatrollingGroup
  (params (InPatrollingGroup :type Byte))
  (Variables|Default|SetPatrollingGroup InPatrollingGroup)
  (if (> (Variables|Default|GetPatrollingGroup) 0)
    (bind _asbp_aicontroller (Utilities|Casting|CastToBP_AIController (AI|GetAIController self)))
    (Default|UpdateAIState _asbp_aicontroller "NewEnumerator1")))

(fn UpdateWeaponMuzzleRotation
  (|CallParentFunction)
  (bind _currentweapon (Variables|Default|GetCurrentWeapon)
    (:then
      (switch Utilities|FlowControl|Switch|SwitchonENUM_WeaponState (Variables|/Game/Blueprints/Weapons/BP_WeaponBase.BP_WeaponBase_C|GetWeaponState _currentweapon)
        (:NewEnumerator0
          (Transformation|SetRelativeRotation (Variables|/Game/Blueprints/Weapons/BP_WeaponBase.BP_WeaponBase_C|GetMuzzleScene (Variables|Default|GetCurrentWeapon)) "0, 0, 0" false false :!label _label))
        (:NewEnumerator1
          (bind _asbp_aicontroller (Utilities|Casting|CastToBP_AIController (Pawn|GetController)))
          (switch Utilities|FlowControl|Switch|SwitchonENUM_AIStates (Variables|/Game/Blueprints/Controllers/BP_AIController.BP_AIController_C|GetAIState _asbp_aicontroller)
            (:NewEnumerator3
              (bind _targetcharacter (Variables|/Game/Blueprints/Controllers/BP_AIController.BP_AIController_C|GetTargetCharacter _asbp_aicontroller)
                (:then
                  (LocalVariables|SetL_TargetLocation (Transformation|GetActorLocation _targetcharacter))
                  (Transformation|SetWorldRotation (Variables|/Game/Blueprints/Weapons/BP_WeaponBase.BP_WeaponBase_C|GetMuzzleScene (Variables|Default|GetCurrentWeapon)) (Math|Rotator|MakeRotator 0.0 (.Pitch (Math|Rotator|BreakRotator (Math|Interpolation|RInterpTo (Transformation|GetWorldRotation (Variables|/Game/Blueprints/Weapons/BP_WeaponBase.BP_WeaponBase_C|GetMuzzleScene (Variables|Default|GetCurrentWeapon))) (Math|Rotator|FindLookatRotation (Transformation|GetWorldLocation (Variables|/Game/Blueprints/Weapons/BP_WeaponBase.BP_WeaponBase_C|GetMuzzleScene (Variables|Default|GetCurrentWeapon))) (LocalVariables|GetL_TargetLocation)) (Utilities|Time|GetWorldDeltaSeconds) 15.0))) (.Yaw (Math|Rotator|BreakRotator (Math|Interpolation|RInterpTo (Transformation|GetWorldRotation (Variables|/Game/Blueprints/Weapons/BP_WeaponBase.BP_WeaponBase_C|GetMuzzleScene (Variables|Default|GetCurrentWeapon))) (Math|Rotator|FindLookatRotation (Transformation|GetWorldLocation (Variables|/Game/Blueprints/Weapons/BP_WeaponBase.BP_WeaponBase_C|GetMuzzleScene (Variables|Default|GetCurrentWeapon))) (LocalVariables|GetL_TargetLocation)) (Utilities|Time|GetWorldDeltaSeconds) 15.0)))) false false))
                (:else)))))
        (:NewEnumerator2
          (goto _label))
        (:NewEnumerator3
          (goto _label))
        (:NewEnumerator4
          (goto _label))))
    (:else)))