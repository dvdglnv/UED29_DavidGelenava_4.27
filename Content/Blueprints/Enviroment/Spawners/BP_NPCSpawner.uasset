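; BP_NPCSpawner is a spawner actor that creates a set number of NPCs of a configurable class at its SpawnPoint.
; Spawning starts on BeginPlay when SpawnOnStart is set, or through StartSpawnNPCs.
; Each spawn assigns any non-zero patrolling group to the NPC, then sets a one-shot timer to space out spawns.
; It finishes when the count is reached or StopSpawnNPCs sets the done flag.
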(event EventBeginPlay
  (if (Variables|Default|GetSpawnOnStart)
    (CallFunction|StartSpawnNPCs)))

(event Collision|EventActorBeginOverlap
  (params (OtherActor :type Actor%20Object%20Reference)))

(event EventTick
  (params (DeltaSeconds :type Float%20%28single-precision%29)))

(fn ConstructionScript)

(fn StartSpawnNPCs
  (CallFunction|SpawnOneNPC))

(fn SpawnOneNPC
  (if (not (Variables|Default|GetIsDone))
    (if (Utilities|IsValidClass (Variables|Default|GetSpawnNPCClass))
      (if (< (Variables|Default|GetCounter) (Variables|Default|GetNPCsCount))
        (bind _returnvalue (Game|SpawnActorfromClass (Variables|Default|GetSpawnNPCClass) (Transformation|GetWorldTransform (Variables|Default|GetSpawnPoint)) "AdjustIfPossibleButAlwaysSpawn" self 0))
        (Variables|Default|SetLastSpawnedNPC _returnvalue)
        (CallFunction|UpdatePatrolStateforSpawnedNPC)
        (Math|Integer|IncrementInt (Variables|Default|GetCounter)
          (:%20%20
            (Utilities|Time|SetTimerbyEvent (EventDispatchers|CreateEvent :!event SpawnOneNPC) (Variables|Default|GetBetweenSpawnDelay))))
        (else
          (Variables|Default|SetIsDone true))))))

(fn StopSpawnNPCs
  (Variables|Default|SetIsDone true))

(fn UpdatePatrolStateforSpawnedNPC
  (if (!= (Variables|Default|GetPatrollingGroup) 0)
    (Default|UpdatePatrollingGroup (Variables|Default|GetLastSpawnedNPC) (Variables|Default|GetPatrollingGroup))))