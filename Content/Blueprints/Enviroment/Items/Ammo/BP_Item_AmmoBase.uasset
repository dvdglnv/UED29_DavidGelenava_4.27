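; Base Blueprint for ammo items that add ammunition to a backpack.
; It overrides PutIntoBackpack to call the parent, then increase the backpack's ammo by its Ammo amount, using ItemName as the weapon name.
; The transfer and the following AfterUse call only happen when the name is set and the amount is positive.
; The event graph and construction script add no logic of their own.
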(event EventBeginPlay
  (|CallParentFunction) ; This node is disabled and will not be called.\nDrag off pins to build functionality.
)

(event Collision|EventActorBeginOverlap
  (params (OtherActor :type Actor%20Object%20Reference))
  (|CallParentFunction OtherActor) ; This node is disabled and will not be called.\nDrag off pins to build functionality.
)

(event EventTick
  (params (DeltaSeconds :type Float%20%28single-precision%29))
  (|CallParentFunction DeltaSeconds) ; This node is disabled and will not be called.\nDrag off pins to build functionality.
)

(fn ConstructionScript
  (|CallParentFunction))

(fn PutIntoBackpack
  (params (InBackpack :type BP%20Backpack%20Component%20Object%20Reference))
  (|CallParentFunction InBackpack)
  (if (and (Utilities|Name|NotEqual(Name) (Variables|Default|GetItemName) "None") (> (Variables|Default|GetAmmo) 0))
    (Default|UpdateAmmobyName InBackpack (Variables|Default|GetItemName) (Variables|Default|GetAmmo) true)
    (CallFunction|AfterUse)))