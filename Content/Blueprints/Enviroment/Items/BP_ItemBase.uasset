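; BP_ItemBase is a base pickup item that bobs and spins in the world and can be put into a player's backpack.
; Overlapping BP_PlayerCharacter shows a text prompt that turns toward the player's camera and enables interaction.
; Interact passes the character's BP_BackpackComponent to PutIntoBackpack, an empty hook here, while AfterUse destroys the actor.
; Tick drives the prompt rotation, constant yaw and eased ping-pong height offset.
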(event EventBeginPlay
  (Rendering|SetVisibility (Variables|Default|GetTextRender) false false)
  (Variables|Default|SetInitialLocation (Transformation|GetWorldLocation (Variables|Default|GetSphereCollision)))
  (Transformation|AddRelativeRotation (Variables|Default|GetSphereCollision) (Math|Rotator|MakeRotator 0.0 0.0 (Math|Random|RandomFloatinRange -9e+01 9e+01)) false false))

(event Collision|EventActorBeginOverlap
  (params (OtherActor :type Actor%20Object%20Reference))
  (bind _asbp_player_character (Utilities|Casting|CastToBP_PlayerCharacter OtherActor))
  (Variables|Use|SetCharacterInBox _asbp_player_character)
  (Rendering|SetVisibility (Variables|Default|GetTextRender) true false)
  (Variables|Use|SetIsReadyToInteract true)
  (Variables|Use|SetIsLookAtPlayerCamera true))

(event Collision|EventActorEndOverlap
  (params (OtherActor :type Actor%20Object%20Reference))
  (Utilities|Casting|CastToBP_PlayerCharacter OtherActor)
  (Variables|Use|SetCharacterInBox 0)
  (Rendering|SetVisibility (Variables|Default|GetTextRender) false false)
  (Variables|Use|SetIsReadyToInteract false)
  (Variables|Use|SetIsLookAtPlayerCamera false))

(event EventTick
  (params (DeltaSeconds :type Float%20%28single-precision%29))
  (Variables|Default|SetDeltaSeconds DeltaSeconds)
  (CallFunction|LookingatPlayerCamera)
  (CallFunction|FloatandRotate))

(fn ConstructionScript)

(fn LookingatPlayerCamera
  (if (Variables|Use|GetIsLookAtPlayerCamera)
    (bind _characterinbox (Variables|Use|GetCharacterInBox)
      (:then
        (bind _asbp_player_character (Utilities|Casting|CastToBP_PlayerCharacter _characterinbox))
        (LocalVariables|SetL_CameraLocation (Transformation|GetWorldLocation (Variables|/Game/Blueprints/Characters/Player/BP_PlayerCharacter.BP_PlayerCharacter_C|GetCamera _asbp_player_character)))
        (Transformation|SetWorldRotation (Variables|Default|GetTextRender) (Math|Rotator|FindLookatRotation (Transformation|GetWorldLocation (Variables|Default|GetTextRender)) (LocalVariables|GetL_CameraLocation)) false false))
      (:else))))

(fn PutIntoBackpack
  (params (InBackpack :type BP%20Backpack%20Component%20Object%20Reference)))

(fn AfterUse
  (Actor|DestroyActor))

(fn FloatandRotate
  (bind _initiallocation (Variables|Default|GetInitialLocation))
  (Utilities|FlowControl|Sequence
    (:then_0
      (if (not (Math|Float|NearlyEqual(Float) (Variables|Default|GetAlphaCurrent) (Math|Float|SelectFloat (Variables|Default|GetAlphaTarger) (Variables|Default|GetAlphaStart) (Variables|Default|GetAlphaForward)) 0.05))
        (Variables|Default|SetAlphaCurrent (Math|Float|ClampAngle (Math|Float|SelectFloat (+ (Variables|Default|GetAlphaCurrent) (Variables|Default|GetDeltaSeconds)) (- (Variables|Default|GetAlphaCurrent) (Variables|Default|GetDeltaSeconds)) (Variables|Default|GetAlphaForward)) 0.0 1.0))
        (else
          (Variables|Default|SetAlphaForward (not (Variables|Default|GetAlphaForward)))))
      (Transformation|SetWorldLocation (Variables|Default|GetSphereCollision) (Math|Interpolation|Ease "EaseInOut" (Variables|Default|GetAlphaCurrent) (Variables|Default|GetInitialLocation) (Math|Vector|MakeVector (.x _initiallocation) (.y _initiallocation) (+ (.z _initiallocation) (Variables|Default|GetLocationOffsetZ))) 2.0) false false))
    (:then_1
      (Transformation|AddRelativeRotation (Variables|Default|GetSphereCollision) (Math|Rotator|MakeRotator 0.0 0.0 (Variables|Default|GetRotationSpeed)) false false))))

(fn Interact
  (if (Variables|Use|GetIsReadyToInteract)
    (bind _characterinbox (Variables|Use|GetCharacterInBox)
      (:then
        (Utilities|IsValid (Actor|GetComponentbyClass _characterinbox "/Game/Blueprints/Components/BP_BackpackComponent.BP_BackpackComponent_C")
          (:Is%20Valid
            (CallFunction|PutIntoBackpack (Actor|GetComponentbyClass _characterinbox "/Game/Blueprints/Components/BP_BackpackComponent.BP_BackpackComponent_C"))
            (return true))
          (:Is%20Not%20Valid
            (return true))))
      (:else
        (return true)))
    (else
      (return true))))