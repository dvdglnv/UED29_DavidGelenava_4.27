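; Destructible helicopter prop that catches fire when its health runs out, then explodes.
; After a delay with fire and light, it briefly expands two damage spheres to hurt characters and fires a radial impulse.
; A BarrelDamage sphere overlap cuts health and jumps into the same destruction sequence, enabling chain reactions.
; The mesh and actor are then destroyed, and BP_Helicopter_Destroy spawns at the saved start location.
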(event OnComponentBeginOverlap(CharacterDamage)
  (params (OverlappedComponent :type Primitive%20Component%20Object%20Reference) (OtherActor :type Actor%20Object%20Reference) (OtherComp :type Primitive%20Component%20Object%20Reference) (OtherBodyIndex :type Integer) (bFromSweep :type Boolean) (SweepResult :type Hit%20Result%20Structure%20%28by%20ref%29))
  ;[1 1 1] Damage to character
  (bind _asbp_character_base (Utilities|Casting|CastToBP_CharacterBase OtherActor))
  (Utilities|FlowControl|DoOnce bFromSweep
    (:Completed
      (Game|Damage|ApplyDamage _asbp_character_base 4e+01 0 OtherActor "/Game/Blueprints/Objects/BP_DamageObject.BP_DamageObject_C"))))

(event OnComponentBeginOverlap(BarrelDamage)
  (params (OverlappedComponent :type Primitive%20Component%20Object%20Reference) (OtherActor :type Actor%20Object%20Reference) (OtherComp :type Primitive%20Component%20Object%20Reference) (OtherBodyIndex :type Integer) (bFromSweep :type Boolean) (SweepResult :type Hit%20Result%20Structure%20%28by%20ref%29))
  ;[1 1 1] Chain reaction
  (Utilities|FlowControl|DoOnce bFromSweep
    (:Completed
      (Variables|Default|SetHelicopterHealth (- (Variables|Default|GetHelicopterHealth) 8e+01))
      (Rendering|SetVisibility (Variables|Default|GetPointLight) true false)
      (Components|Activation|Activate (Variables|Default|GetFireVFX) false)
      (Utilities|FlowControl|Delay 4.0)
      (Utilities|IsValid (Variables|Default|GetCharacterDamage)
        (:Is%20Valid
          (Audio|SpawnSoundatLocation "/Game/StarterContent/Audio/Explosion_Cue.Explosion_Cue" "0, 0, 0" "0, 0, 0" 5.0 1.0 0.0 0 0)
          (Components|Activation|Activate (Variables|Default|GetCharacterDamage) false)
          (Components|Activation|Activate (Variables|Default|GetBarrelDamage) false)
          (Components|Sphere|SetSphereRadius (Variables|Default|GetCharacterDamage) 5e+02 true)
          (Components|Sphere|SetSphereRadius (Variables|Default|GetBarrelDamage) 5e+02 true)
          (Components|DestroyComponent (Variables|Default|GetCharacterDamage))
          (Class|RadialForceComponent|FireImpulse (Variables|Default|GetRadialForce))
          (Components|Activation|Activate (Variables|Default|GetExplosionVFX) false))
        (:Is%20Not%20Valid
          _))
      (Utilities|IsValid (Variables|Default|GetHelicopterMesh)
        (:Is%20Valid
          (Components|DestroyComponent (Variables|Default|GetHelicopterMesh))
          (Components|Activation|Deactivate (Variables|Default|GetFireVFX))
          (Rendering|SetVisibility (Variables|Default|GetPointLight) false false)
          (Utilities|FlowControl|Delay 0.2)
          (Actor|DestroyActor)
          (Game|SpawnActorfromClass "/Game/Blueprints/Enviroment/BP_Helicopter_Destroy.BP_Helicopter_Destroy_C" (Math|Conversions|ToTransform(Vector) (Variables|Default|GetSpawnLocation)) "AdjustIfPossibleButAlwaysSpawn" "MultiplyWithRoot" 0 0))))))

(event EventBeginPlay
  (Components|Sphere|SetSphereRadius (Variables|Default|GetBarrelDamage) 0.0 true)
  (Components|Sphere|SetSphereRadius (Variables|Default|GetCharacterDamage) 0.0 true)
  (Components|Activation|Deactivate (Variables|Default|GetBarrelDamage))
  (Components|Activation|Deactivate (Variables|Default|GetCharacterDamage))
  (Transformation|SetWorldLocation (Variables|Default|GetHelicopterMesh) (Transformation|GetWorldLocation (Variables|Default|GetHelicopterMesh)) false false)
  (Variables|Default|SetSpawnLocation (Transformation|GetWorldLocation (Variables|Default|GetHelicopterMesh))))

(event Game|Damage|EventAnyDamage
  (params (Damage :type Float%20%28single-precision%29) (DamageType :type Damage%20Type%20Object%20Reference) (InstigatedBy :type Controller%20Object%20Reference) (DamageCauser :type Actor%20Object%20Reference))
  (bind _output_get (Variables|Default|SetHelicopterHealth (- (Variables|Default|GetHelicopterHealth) Damage)))
  (if (<= _output_get 1.0)
    (Rendering|SetVisibility (Variables|Default|GetPointLight) true false)
    (Components|Activation|Activate (Variables|Default|GetFireVFX) false)
    (Utilities|FlowControl|Delay 4.0)
    (Utilities|IsValid (Variables|Default|GetCharacterDamage)
      (:Is%20Valid
        (Audio|SpawnSoundatLocation "/Game/StarterContent/Audio/Explosion_Cue.Explosion_Cue" "0, 0, 0" "0, 0, 0" 5.0 1.0 0.0 0 0)
        (Components|Activation|Activate (Variables|Default|GetCharacterDamage) false)
        (Components|Activation|Activate (Variables|Default|GetBarrelDamage) false)
        (Components|Sphere|SetSphereRadius (Variables|Default|GetCharacterDamage) 5e+02 true)
        (Components|Sphere|SetSphereRadius (Variables|Default|GetBarrelDamage) 5e+02 true)
        (Components|DestroyComponent (Variables|Default|GetCharacterDamage))
        (Class|RadialForceComponent|FireImpulse (Variables|Default|GetRadialForce))
        (Components|Activation|Activate (Variables|Default|GetExplosionVFX) false))
      (:Is%20Not%20Valid
        _))
    (Utilities|IsValid (Variables|Default|GetHelicopterMesh)
      (:Is%20Valid
        (Components|DestroyComponent (Variables|Default|GetHelicopterMesh))
        (Components|Activation|Deactivate (Variables|Default|GetFireVFX))
        (Rendering|SetVisibility (Variables|Default|GetPointLight) false false)
        (Utilities|FlowControl|Delay 0.2)
        (Actor|DestroyActor)
        (Game|SpawnActorfromClass "/Game/Blueprints/Enviroment/BP_Helicopter_Destroy.BP_Helicopter_Destroy_C" (Math|Conversions|ToTransform(Vector) (Variables|Default|GetSpawnLocation)) "AdjustIfPossibleButAlwaysSpawn" "MultiplyWithRoot" 0 0)))))

(fn ConstructionScript)