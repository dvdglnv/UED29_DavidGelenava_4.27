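; Double door Blueprint for the lab environment that swings two door rotators open and closed.
; Two custom events play or reverse a timeline, which sets the same relative yaw on both rotators, scaled by the maximum open angle.
; An in-progress flag blocks retriggering mid-swing, and the timeline's finish direction sets the open state.
; Despite the asset name, these graphs contain no lock logic.
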(event Custom|CustomEvent
  (if (not (Variables|Default|GetInProgress))
    (if (not (Variables|Default|GetIsDoorOpen))
      (bind (_direction _openprogression) (Timeline|Timeline PlayFromStart)
        (:Update
          (Variables|Default|SetInProgress true)
          (Transformation|SetRelativeRotation (Variables|Default|GetDoorRotator) (Math|Rotator|MakeRotator 0.0 0.0 (* (Variables|Default|GetMaxDoorOpenAngle) _openprogression)) false false))
        (:Finished
          (Variables|Default|SetInProgress false)
          (switch Utilities|FlowControl|Switch|SwitchonETimelineDirection _direction
            (:Forward
              (Variables|Default|SetIsDoorOpen true))
            (:Backward
              (Variables|Default|SetIsDoorOpen false))))))))

(event Custom|CustomEvent_1
  (if (not (Variables|Default|GetInProgress))
    (if (Variables|Default|GetIsDoorOpen)
      (bind (_direction _openprogression) (Timeline|Timeline ReverseFromEnd)
        (:Update
          (Variables|Default|SetInProgress true)
          (Transformation|SetRelativeRotation (Variables|Default|GetDoorRotator) (Math|Rotator|MakeRotator 0.0 0.0 (* (Variables|Default|GetMaxDoorOpenAngle) _openprogression)) false false))
        (:Finished
          (Variables|Default|SetInProgress false)
          (switch Utilities|FlowControl|Switch|SwitchonETimelineDirection _direction
            (:Forward
              (Variables|Default|SetIsDoorOpen true))
            (:Backward
              (Variables|Default|SetIsDoorOpen false))))))))

(event EventBeginPlay
  (|CallParentFunction) ; This node is disabled and will not be called.\nDrag off pins to build functionality.
)

(event Collision|EventActorBeginOverlap
  (params (OtherActor :type Actor%20Object%20Reference))
  (|CallParentFunction OtherActor) ; This node is disabled and will not be called.\nDrag off pins to build functionality.
)

(event EventTick
  (params (DeltaSeconds :type Float%20%28single-precision%29))
  (|CallParentFunction DeltaSeconds) ; This node is disabled and will not be called.\nDrag off pins to build functionality.
)

(fn ConstructionScript
  (|CallParentFunction))