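; Tooltip actor variant whose text turns to face the player's camera while the player is in its overlap area.
; Begin overlap runs the parent logic, then enables look-at if PlayerInBox is valid; any end overlap disables it.
; While enabled, Tick rotates TooltipText toward the BP_PlayerCharacter camera using FindLookAtRotation.
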(event EventBeginPlay
  (|CallParentFunction) ; This node is disabled and will not be called.\nDrag off pins to build functionality.
)

(event Collision|EventActorBeginOverlap
  (params (OtherActor :type Actor%20Object%20Reference))
  (|CallParentFunction OtherActor) ; This node is disabled and will not be called.\nDrag off pins to build functionality.
)

(event EventTick
  (params (DeltaSeconds :type Float%20%28single-precision%29))
  (|CallParentFunction DeltaSeconds)
  (CallFunction|LookingatPlayerCaamera))

(event EventActorBeginOverlap
  (params (OtherActor :type Actor%20Object%20Reference))
  (|CallParentFunction OtherActor)
  (Variables|Default|GetPlayerInBox
    (:then
      (Variables|Default|SetIsLookAtPlayerCamera true))
    (:else)))

(event EventActorEndOverlap
  (params (OtherActor :type Actor%20Object%20Reference))
  (|CallParentFunction OtherActor)
  (Variables|Default|SetIsLookAtPlayerCamera false))

(fn ConstructionScript
  (|CallParentFunction))

(fn LookingatPlayerCaamera
  (if (Variables|Default|GetIsLookAtPlayerCamera)
    (bind _playerinbox (Variables|Default|GetPlayerInBox)
      (:then
        (bind _asbp_player_character (Utilities|Casting|CastToBP_PlayerCharacter _playerinbox))
        (LocalVariables|SetL_CameraLocation (Transformation|GetWorldLocation (Variables|/Game/Blueprints/Characters/Player/BP_PlayerCharacter.BP_PlayerCharacter_C|GetCamera _asbp_player_character)))
        (Transformation|SetWorldRotation (Variables|Default|GetTooltipText) (Math|Rotator|FindLookatRotation (Transformation|GetWorldLocation (Variables|Default|GetTooltipText)) (LocalVariables|GetL_CameraLocation)) false false))
      (:else))))