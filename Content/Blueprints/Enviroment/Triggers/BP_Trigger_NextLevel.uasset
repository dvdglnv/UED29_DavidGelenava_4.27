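; Level-transition trigger that advances the game to the next level when the player enters it.
; On overlap it runs the parent trigger logic, then casts OverlappedActor to BP_PlayerCharacter, falling back to BP_VehicleBase.
; Either match calls UpdateNextLevel on BP_GameInstance through a DoOnce, so it fires only once.
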(event EventBeginPlay
  (|CallParentFunction) ; This node is disabled and will not be called.\nDrag off pins to build functionality.
)

(event Collision|EventActorBeginOverlap
  (params (OtherActor :type Actor%20Object%20Reference))
  (bind _overlappedactor (Variables|Default|GetOverlappedActor))
  (|CallParentFunction OtherActor)
  (Utilities|Casting|CastToBP_PlayerCharacter _overlappedactor
    (:then
      _)
    (:CastFailed
      (Utilities|Casting|CastToBP_VehicleBase _overlappedactor)))
  (bind _asbp_game_instance (Utilities|Casting|CastToBP_GameInstance (Game|GetGameInstance)))
  (Utilities|FlowControl|DoOnce false
    (:Completed
      (Default|UpdateNextLevel _asbp_game_instance))))

(event EventTick
  (params (DeltaSeconds :type Float%20%28single-precision%29))
  (|CallParentFunction DeltaSeconds) ; This node is disabled and will not be called.\nDrag off pins to build functionality.
)

(fn ConstructionScript
  (|CallParentFunction))