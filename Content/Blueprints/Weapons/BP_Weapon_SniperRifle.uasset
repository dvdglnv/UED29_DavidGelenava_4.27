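; Sniper rifle weapon that overrides the parent's single shot with a hitscan trace and adds a laser sight.
; Shots trace from the muzzle with debug drawing, triple damage on "head" bone hits, attach a randomly rolled impact effect to the hit component, and always play shot effects.
; Each tick, a second trace stretches the laser mesh and moves its point light to the hit; weapon activation toggles that light's visibility.
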(event EventBeginPlay
  (|CallParentFunction)
  (AimLaser|AimLaserConfigure))

(event Collision|EventActorBeginOverlap
  (params (OtherActor :type Actor%20Object%20Reference))
  (|CallParentFunction OtherActor) ; This node is disabled and will not be called.\nDrag off pins to build functionality.
)

(event EventTick
  (params (DeltaSeconds :type Float%20%28single-precision%29))
  (|CallParentFunction DeltaSeconds)
  (AimLaser|AimLaserUpdate))

(fn ConstructionScript
  (|CallParentFunction))

(fn ConfigureWeaponStats
  (params (IsWeaponName :type Name :default "None"))
  (|CallParentFunction IsWeaponName))

(fn SingleShot
  (bind _muzzlescene (Variables|Default|GetMuzzleScene))
  (bind _returnvalue (Transformation|GetWorldLocation _muzzlescene))
  (Utilities|FlowControl|Sequence
    (:then_0
      (bind (_outhit _returnvalue_2) (Collision|LineTraceByChannel _returnvalue (+ _returnvalue (* (Math|Vector|GetForwardVector (Variables|Default|GetMuzzleScene)) 2.5e+04)) "TraceTypeQuery2" true (Utilities|Array|MakeArray self (Components|GetOwner)) "ForDuration" true "(R=1.000000,G=0.000000,B=0.000000,A=1.000000)" "(R=0.000000,G=1.000000,B=0.000000,A=1.000000)" 3.0))
      (if _returnvalue_2
        (Variables|Default|SetHitResult _outhit)
        (Variables|Default|SetHitLocation (.Location (Collision|BreakHitResult (Variables|Default|GetHitResult))))
        (Variables|Default|SetHitNormal (.Normal (Collision|BreakHitResult (Variables|Default|GetHitResult))))
        (Variables|Default|SetHitActor (.HitActor (Collision|BreakHitResult (Variables|Default|GetHitResult))))
        (Variables|Default|SetHitComponent (.HitComponent (Collision|BreakHitResult (Variables|Default|GetHitResult))))
        (Utilities|FlowControl|Sequence
          (:then_0
            (CallFunction|ApplyDamagebyHitScan))
          (:then_1
            (CallFunction|SpawnDecal)))))
    (:then_1
      (CallFunction|ShotEffects))))

(fn ApplyDamagebyHitScan
  (Utilities|FlowControl|Sequence
    (:then_0
      (LocalVariables|SetL_Damage (Variables|Default|GetDamageCurrent)))
    (:then_1
      (if (Utilities|Name|Equal(Name) (.HitBoneName (Collision|BreakHitResult (Variables|Default|GetHitResult))) "head")
        (LocalVariables|SetL_Damage (* (LocalVariables|GetL_Damage) 3))))
    (:then_2
      (Game|Damage|ApplyDamage (Variables|Default|GetHitActor) (Math|Conversions|ToFloat(Integer) (LocalVariables|GetL_Damage)) 0 (Components|GetOwner) "/Game/Blueprints/Objects/BP_DamageObject.BP_DamageObject_C"))))

(fn SpawnDecal
  (bind _hitnormal (Variables|Default|GetHitNormal))
  (bind _returnvalue (Math|Conversions|RotationFromXVector _hitnormal))
  (LocalVariables|SetL_Rotator (Math|Rotator|MakeRotator (Math|Random|RandomFloatinRange 0.0 3.6e+02) (.pitch _returnvalue) (.yaw _returnvalue)))
  (bind _returnvalue_2 (Game|SpawnActorfromClass "/Game/Blueprints/Weapons/Projectiles/BP_ImpactEffect.BP_ImpactEffect_C" (Math|Transform|MakeTransform (Variables|Default|GetHitLocation) (LocalVariables|GetL_Rotator) "1.000000,1.000000,1.000000") "Undefined" "OverrideRootScale" self 0))
  (LocalVariables|SetL_Impact _returnvalue_2)
  (Transformation|AttachComponentToComponent (LocalVariables|GetL_Impact) (Variables|Default|GetHitComponent) (.HitBoneName (Collision|BreakHitResult (Variables|Default|GetHitResult))) "KeepWorld" "KeepWorld" "KeepWorld" true))

(fn AimLaserConfigure
  (Components|StaticMesh|SetStaticMesh (Variables|Default|GetAimLaserStaticMesh) (Variables|Default|GetAimSM))
  (Rendering|Material|SetMaterial (Variables|Default|GetAimLaserStaticMesh) 0 (Variables|Default|GetAimMI)))

(fn AimLaserUpdate
  (bind _aimlaser (Variables|Default|GetAimLaser))
  (bind _aimlaserstaticmesh (Variables|Default|GetAimLaserStaticMesh))
  (bind _aimlaserstaticmesh_2 (Variables|Default|GetAimLaserStaticMesh))
  (bind _returnvalue (Transformation|GetWorldLocation _aimlaser))
  (bind _returnvalue_2 (Transformation|GetWorldScale _aimlaserstaticmesh_2))
  (bind _returnvalue_3 (Transformation|GetWorldScale _aimlaserstaticmesh))
  (bind (_outhit _returnvalue_4) (Collision|LineTraceByChannel _returnvalue (+ _returnvalue (* (Math|Vector|GetForwardVector _aimlaser) 5e+03)) "TraceTypeQuery2" true 0 "None"))
  (if _returnvalue_4
    (LocalVariables|SetL_Distance (.Distance (Collision|BreakHitResult _outhit)))
    (LocalVariables|SetL_Location (.Location (Collision|BreakHitResult _outhit)))
    (Transformation|SetWorldScale3D (Variables|Default|GetAimLaserStaticMesh) (Math|Vector|MakeVector (/ (LocalVariables|GetL_Distance) 1e+03) (.y _returnvalue_3) (.z _returnvalue_3)))
    (Transformation|SetWorldLocation (Variables|Default|GetAimLaserPointLight) (LocalVariables|GetL_Location) false false)
    (Rendering|Components|Light|SetIntensity (Variables|Default|GetAimLaserPointLight) 1e+03)
    (else
      (Transformation|SetWorldScale3D _aimlaserstaticmesh_2 (Math|Vector|MakeVector 1.0 (.y _returnvalue_2) (.z _returnvalue_2)))
      (Transformation|SetWorldLocation (Variables|Default|GetAimLaserPointLight) (Transformation|GetWorldLocation (Variables|Default|GetAimLaser)) false false)
      (Rendering|Components|Light|SetIntensity (Variables|Default|GetAimLaserPointLight) 1e+02))))

(fn ActivateWeapon
  (params (InActivation :type Boolean))
  (|CallParentFunction InActivation)
  (Rendering|SetVisibility (Variables|Default|GetAimLaserPointLight) InActivation false))